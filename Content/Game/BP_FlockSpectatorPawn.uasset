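; Top-down spectator pawn for viewing a flock scene from high above and placing spawns.
; Enhanced Input drives planar movement and scroll zoom, with Tick easing height toward the scrolled target.
; Dragging pans by intersecting mouse rays with the Z=0 plane and offsetting from the cached grab point.
; Left click moves the BP_SmallSpawner found in the level to the ground under the cursor and triggers DoSpawning.
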(event Input|EnhancedActionEvents|EnhancedInputActionIA_Scroll
  (params (ActionValue :type Float%20%28double-precision%29) (ElapsedSeconds :type Float%20%28double-precision%29) (TriggeredSeconds :type Float%20%28double-precision%29) (InputAction :type Input%20Action%20Object%20Reference :default "/Game/Game/Input/InputActions/IA_Scroll.IA_Scroll"))
  (:Triggered
    (Variables|Default|SetDesired%20Location (+ (Variables|Default|GetDesired%20Location) (* ActionValue (Utilities|Time|GetWorldDeltaSeconds) (Math|Vector|MakeVector 0.0 0.0 2e+05))))))

(event Input|EnhancedActionEvents|EnhancedInputActionIA_Move
  (params (ActionValue :type Vector%202D%20Structure) (ElapsedSeconds :type Float%20%28double-precision%29) (TriggeredSeconds :type Float%20%28double-precision%29) (InputAction :type Input%20Action%20Object%20Reference :default "/Game/Game/Input/InputActions/IA_Move.IA_Move"))
  (:Triggered
    (Transformation|SetActorLocation (+ (Transformation|GetActorLocation) (* (Math|Vector2D|Normalize2D ActionValue) (Utilities|Time|GetWorldDeltaSeconds) 1e+01)) false true)))

(event Input|EnhancedActionEvents|EnhancedInputActionIA_Drag
  (params (ActionValue :type Boolean) (ElapsedSeconds :type Float%20%28double-precision%29) (TriggeredSeconds :type Float%20%28double-precision%29) (InputAction :type Input%20Action%20Object%20Reference :default "/Game/Game/Input/InputActions/IA_Drag.IA_Drag"))
  (bind _returnvalue (Transformation|GetActorLocation))
  (bind _returnvalue_2 (Class|KismetMathLibrary|MakePlanefromPointandNormal "0, 0, 0" "0.000000,0.000000,1.000000"))
  (bind _returnvalue_3 (Game|GetPlayerController 0))
  (bind _worldlocation (Game|Player|ConvertMouseLocationToWorldSpace _returnvalue_3))
  (bind _returnvalue_4 (- _worldlocation _returnvalue))
  (bind _returnvalue_5 (* _returnvalue_4 2e+05))
  (bind _intersection (Class|KismetMathLibrary|LinePlaneIntersection _returnvalue _returnvalue_5 _returnvalue_2))
  (:Triggered
    (Transformation|SetActorLocation (+ (- (Variables|Default|GetCached%20Location) _intersection) (Transformation|GetActorLocation)) false true))
  (:Started
    (Variables|Default|SetCached%20Location _intersection)))

(event EventBeginPlay
  (bind _output_get (Variables|Default|SetDesired%20Location "0.000000,0.000000,35000.000000"))
  (Transformation|SetActorLocation _output_get false true)
  (Transformation|SetActorRotation "-90.000000,0.000000,0.000000"))

(event Collision|EventActorBeginOverlap
  (params (OtherActor :type Actor%20Object%20Reference)))

(event EventTick
  (params (DeltaSeconds :type Float%20%28single-precision%29))
  (bind _returnvalue (Transformation|GetActorLocation))
  (Transformation|SetActorLocation (Math|Vector|MakeVector (.x _returnvalue) (.y _returnvalue) (Class|KismetMathLibrary|FInterpEaseinOut (.z _returnvalue) (.z (Variables|Default|GetDesired%20Location)) DeltaSeconds 0.5)) false true))

(event Input|MouseEvents|LeftMouseButton
  (params (Key :type Key%20Structure :default "None"))
  (bind _returnvalue (Game|GetPlayerController 0))
  (bind (_locationx _locationy) (Game|Player|GetMousePosition _returnvalue))
  (:Pressed
    (bind _returnvalue_2 (Actor|GetActorOfClass "/Game/Game/BP_SmallSpawner.BP_SmallSpawner_C"))
    (Transformation|SetActorLocation _returnvalue_2 (Class|FlockBlueprintFunctionLibrary|DeprojectScreenPositiontoGround _returnvalue _locationx _locationy 0.0) false true)
    (Class|MassSpawner|DoSpawning _returnvalue_2)))

(fn ConstructionScript)